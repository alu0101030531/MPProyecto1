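; Bullet is a projectile actor that damages and knocks back third-person characters near its point of impact.
; When its sphere component hits something, a small sphere overlap finds nearby BP_ThirdPersonCharacter pawns and calls ReceiveShot on each.
; Each call passes Damage and an impulse pointing away from the bullet, scaled by EfectoImpacto.
; It then spawns the EM_Impact_System effect at its location and destroys itself.
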(event `self.Sphere.OnComponentHit`
  (params (HitComponent :type "PrimitiveComponent Object Reference") (OtherActor :type "Actor Object Reference") (OtherComp :type "PrimitiveComponent Object Reference") (NormalImpulse :type "Vector Structure") (Hit :type "HitResult Structure (by ref)"))
  ;[0.353 1 0.1284] Impacto
  (bind _outactors (`KismetSystemLibrary.SphereOverlapActors` (`self.K2_GetActorLocation`) 50.0 (`|MakeArray` "ObjectTypeQuery3" :!type "EObjectTypeQuery Enum") "/Game/ThirdPerson/Blueprints/BP_ThirdPersonCharacter.BP_ThirdPersonCharacter_C"))
  (for _array_element _outactors
    (bind _asbp_third_person_character (cast `/Game/ThirdPerson/Blueprints/BP_ThirdPersonCharacter` _array_element))
    (`/Game/ThirdPerson/Blueprints/BP_ThirdPersonCharacter.ReceiveShot` _asbp_third_person_character (`self.Damage`) (* (`KismetMathLibrary.GetDirectionUnitVector` (`self.K2_GetActorLocation`) (`self.K2_GetActorLocation` _array_element)) (`self.EfectoImpacto`))))
  (`self.StartImpactEffect`)
  (`self.K2_DestroyActor`))

(event `StartImpactEffect`
  (`NiagaraFunctionLibrary.SpawnSystemAtLocation` "/Game/Efectos/EM_Impact_System.EM_Impact_System" (`self.K2_GetActorLocation`)))

(fn `UserConstructionScript`)